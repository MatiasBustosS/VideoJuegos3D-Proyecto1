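; BP_Enemigo2 is an enemy variant that sets its own Life and Speed on BeginPlay, then calls the parent's BeginPlay.
; Each Tick runs the parent logic first, then spawns a BP_Mancha whenever the CrearMancha flag is true.
; The spawned BP_Mancha takes its X and Y from the Location variable and uses a fixed height.
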(event EventBeginPlay
  (Variables|Default|SetLife 2)
  (Variables|Default|SetSpeed 2.5e+02)
  (|CallParentFunction))

(event Collision|EventActorBeginOverlap
  (params (OtherActor :type Actor%20Object%20Reference))
  (|CallParentFunction OtherActor) ; This node is disabled and will not be called.\nDrag off pins to build functionality.
)

(event EventTick
  (params (DeltaSeconds :type Float%20%28single-precision%29))
  (bind _location (Variables|Default|GetLocation))
  (|CallParentFunction DeltaSeconds)
  (if (Variables|Default|GetCrearMancha)
    (Game|SpawnActorfromClass "/Game/Enemigos/Mancha/BP_Mancha.BP_Mancha_C" (Math|Conversions|ToTransform(Vector) (Math|Vector|MakeVector (.x _location) (.y _location) 161.0)) "Undefined" 0 0)))

(fn ConstructionScript
  (|CallParentFunction))