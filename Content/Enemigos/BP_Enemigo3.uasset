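; BP_Enemigo3 is an enemy Blueprint that splits into two BP_Enemigo1 enemies when destroyed.
; BeginPlay sets its Life and Speed before calling the parent implementation, which leaves any further behavior to the parent class.
; The Destroyed event spawns both replacements from a Location value, without calling the parent event.
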(event EventBeginPlay
  (Variables|Default|SetLife 3)
  (Variables|Default|SetSpeed 1e+02)
  (|CallParentFunction))

(event Collision|EventActorBeginOverlap
  (params (OtherActor :type Actor%20Object%20Reference))
  (|CallParentFunction OtherActor) ; This node is disabled and will not be called.\nDrag off pins to build functionality.
)

(event EventTick
  (params (DeltaSeconds :type Float%20%28single-precision%29))
  (|CallParentFunction DeltaSeconds) ; This node is disabled and will not be called.\nDrag off pins to build functionality.
)

(event EventDestroyed
  (Game|SpawnActorfromClass "/Game/Enemigos/BP_Enemigo1.BP_Enemigo1_C" (Math|Conversions|ToTransform(Vector) (Variables|Default|GetLocation)) "Undefined" 0 0)
  (Game|SpawnActorfromClass "/Game/Enemigos/BP_Enemigo1.BP_Enemigo1_C" (Math|Conversions|ToTransform(Vector) (Variables|Default|GetLocation)) "Undefined" 0 0))

(fn ConstructionScript
  (|CallParentFunction))