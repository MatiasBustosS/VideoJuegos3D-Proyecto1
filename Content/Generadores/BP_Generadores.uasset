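; BP_Generadores is an enemy spawner that emits timed waves of three enemy types at its own location.
; Tick calls Generar every frame, relying on latent Delays to pace the staggered spawns, with a Start flag skipping the first wait.
; VerOleada shortens the interval after every third wave.
; When the interval runs out, it sets Enabled on the player's TwinStickPawn and destroys itself.
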(event Custom|Generar
  (bind _returnvalue (Transformation|GetActorLocation))
  (if (Variables|Default|GetStart)
    (Variables|Default|SetStart false)
    (else
      (Utilities|FlowControl|Delay (Variables|Default|GetTimeToSpawn))))
  (Game|SpawnActorfromClass "/Game/Enemigos/BP_Enemigo3.BP_Enemigo3_C" (Math|Conversions|ToTransform(Vector) _returnvalue) "AdjustIfPossibleButAlwaysSpawn" 0 0)
  (Utilities|FlowControl|Delay 0.35)
  (Game|SpawnActorfromClass "/Game/Enemigos/BP_Enemigo2.BP_Enemigo2_C" (Math|Conversions|ToTransform(Vector) _returnvalue) "AdjustIfPossibleButAlwaysSpawn" 0 0)
  (Utilities|FlowControl|Delay 0.35)
  (Game|SpawnActorfromClass "/Game/Enemigos/BP_Enemigo1.BP_Enemigo1_C" (Math|Conversions|ToTransform(Vector) _returnvalue) "AdjustIfPossibleButAlwaysSpawn" 0 0)
  (CallFunction|VerOleada))

(event Custom|Ver%20Oleada
  (Variables|Default|SetOleada (+ (Variables|Default|GetOleada) 1))
  (if (>= (Variables|Default|GetOleada) 3)
    (Variables|Default|SetOleada 0)
    (bind _output_get (Variables|Default|SetTimeToSpawn (- (Variables|Default|GetTimeToSpawn) 1.0)))
    (if (<= _output_get 0.0)
      (bind _astwin_stick_pawn (Utilities|Casting|CastToTwinStickPawn (Game|Player|GetPlayerPawn 0)))
      (Variables|/Game/TwinStickBP/Blueprints/TwinStickPawn.TwinStickPawn_C|SetEnabled _astwin_stick_pawn true)
      (Actor|DestroyActor))))

(event EventBeginPlay
  (Variables|Default|SetOleada 0)
  (Variables|Default|SetTimeToSpawn 2.0))

(event EventTick
  (params (DeltaSeconds :type Float%20%28single-precision%29))
  (CallFunction|Generar))

(fn ConstructionScript)